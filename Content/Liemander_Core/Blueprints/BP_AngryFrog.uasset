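; BP_AngryFrog is a frog enemy that fires projectiles at the player's BP_MainGirl pawn, which it caches on BeginPlay.
; Each tick, while alive, allowed to attack and reloaded, it spawns a BP_FrogProjectile and launches its mesh toward the girl with a physics impulse, then reloads through a Delay.
; The head mesh turns toward the girl every tick regardless of state, applying a world-space look-at as relative rotation.
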(event `self.ReceiveBeginPlay`
  (bind _asbp_main_girl (cast `/Game/Liemander_Core/MainGirl/BP_MainGirl` (`GameplayStatics.GetPlayerPawn` 0)))
  (set `self.Target Girl` _asbp_main_girl))

(event `self.ReceiveTick`
  (params (DeltaSeconds :type "Float (single-precision)"))
  (`|ExecutionSequence`
    (:`then_0`
      (if (`self.IsDead`)
        _
        (elif (`self.isCanAttack`)
          (if (`self.isReloadDefaultAttack`)
            (bind _returnvalue (`|SpawnActorFromClass` "/Game/Liemander_Core/Blueprints/BP_FrogProjectile.BP_FrogProjectile_C" (`KismetMathLibrary.Conv_VectorToTransform` (`SceneComponent.K2_GetComponentLocation` (`self.SpawnFrogProj`))) "Undefined" "OverrideRootScale" null null))
            (`PrimitiveComponent.AddImpulse` (`/Game/Liemander_Core/Blueprints/BP_FrogProjectile.StaticMesh` _returnvalue) (* (`KismetMathLibrary.GetForwardVector` (`KismetMathLibrary.FindLookAtRotation` (`SceneComponent.K2_GetComponentLocation` (`self.SpawnFrogProj`)) (`self.K2_GetActorLocation` (`self.Target Girl`)))) 100000.0) "None" false)
            (set `self.isReloadDefaultAttack` false)
            (`KismetSystemLibrary.Delay` 1.5)
            (set `self.isReloadDefaultAttack` true)))))
    (:`then_1`
      (`SceneComponent.K2_SetRelativeRotation` (`self.SM_FrogHead`) (`KismetMathLibrary.FindLookAtRotation` (`SceneComponent.GetSocketLocation` (`self.SM_FrogHead`) "None") (`self.K2_GetActorLocation` (`self.Target Girl`))) false false))))

(fn `UserConstructionScript`)
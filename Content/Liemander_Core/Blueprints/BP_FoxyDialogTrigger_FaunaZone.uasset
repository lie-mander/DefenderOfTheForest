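; BP_FoxyDialogTrigger_FaunaZone is a hidden trigger volume that starts the fox's fauna-zone dialog when BP_MainGirl enters.
; On BeginPlay it initializes the main controller's fox fauna trigger and hooks BP_MainHUD's widgets-created event to bind to WBP_Dialogs.
; Overlap tracks range and calls the fauna dialog unless blocked or CheckFirstDialog is set.
; Handlers for clearing that flag and blocking the trigger accompany bindings to first-dialog and fauna-dialog end events.
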(event `self.ReceiveBeginPlay`
  (bind _asbp_main_hud (cast `/Game/Liemander_Core/Widgets/BP_MainHUD` (`PlayerController.GetHUD` (`GameplayStatics.GetPlayerController` 0))))
  (add `/Game/Liemander_Core/Widgets/BP_MainHUD.WidgetsCreated` _asbp_main_hud (`|CreateDelegate` :!event `WidgetsInit`))
  (bind _asbp_main_controller (cast `/Game/Liemander_Core/MainGirl/BP_MainController` (`GameplayStatics.GetPlayerController` 0)))
  (`/Game/Liemander_Core/MainGirl/BP_MainController.InitializeFoxFaunaTrigger` _asbp_main_controller)
  (bind _asbp_main_hud_2 (cast `/Game/Liemander_Core/Widgets/BP_MainHUD` (`PlayerController.GetHUD` (`GameplayStatics.GetPlayerController` 0))))
  (add `/Game/Liemander_Core/Widgets/BP_MainHUD.WidgetsCreated` _asbp_main_hud_2 (`|CreateDelegate` :!event `BindFaunaDialog`)))

(event `BindFaunaDialog`
  (bind _foundwidgets (`WidgetBlueprintLibrary.GetAllWidgetsOfClass` "/Game/Liemander_Core/Widgets/WBP_Dialogs.WBP_Dialogs_C"))
  (`/Game/Liemander_Core/Widgets/WBP_Dialogs.BindFaunaDialog` (`|GetArrayItem` _foundwidgets)))

(event `WidgetsInit`
  (bind _foundwidgets (`WidgetBlueprintLibrary.GetAllWidgetsOfClass` "/Game/Liemander_Core/Widgets/WBP_Dialogs.WBP_Dialogs_C" false))
  (bind _output (`|GetArrayItem` _foundwidgets))
  (add `/Game/Liemander_Core/Widgets/WBP_Dialogs.FirstDialogEnd` _output (`|CreateDelegate` :!event `SetCheckFirstDialog`))
  (add `/Game/Liemander_Core/Widgets/WBP_Dialogs.FaunaDialogEnd` _output (`|CreateDelegate` :!event `BlockDialogTrigger`)))

(event `SetCheckFirstDialog`
  (set `self.CheckFirstDialog` false))

(event `BlockDialogTrigger`
  (set `self.IsBlock` true))

(event `self.Trigger.OnComponentBeginOverlap`
  (params (OverlappedComponent :type "PrimitiveComponent Object Reference") (OtherActor :type "Actor Object Reference") (OtherComp :type "PrimitiveComponent Object Reference") (OtherBodyIndex :type Integer) (bFromSweep :type Boolean) (SweepResult :type "HitResult Structure (by ref)"))
  (if (not (`self.IsBlock`))
    (cast `/Game/Liemander_Core/MainGirl/BP_MainGirl` OtherActor)
    (set `self.InRangeFaunaDialog` true)
    (if (not (`self.CheckFirstDialog`))
      (`self.eFaunaDialog`)
      (set `self.CanFaunaDialog` true))))

(event `self.Trigger.OnComponentEndOverlap`
  (params (OverlappedComponent :type "PrimitiveComponent Object Reference") (OtherActor :type "Actor Object Reference") (OtherComp :type "PrimitiveComponent Object Reference") (OtherBodyIndex :type Integer))
  (cast `/Game/Liemander_Core/MainGirl/BP_MainGirl` OtherActor)
  (set `self.InRangeFaunaDialog` false))

(fn `UserConstructionScript`
  (`SceneComponent.SetVisibility` (`self.Trigger`) false false))
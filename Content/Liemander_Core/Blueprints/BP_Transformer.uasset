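; BP_Transformer is an interactable transformer that the player breaks to damage the BP_AngryFrog boss.
; A trigger overlap with BP_MainGirl shows a button, which yaws toward her every tick, and arms activation through the controller's ActivateButton event dispatcher.
; Activation subtracts one frog health, flags death with large sparks at zero, then plays break sounds and destroys the transformer.
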(event `self.ReceiveTick`
  (params (DeltaSeconds :type "Float (single-precision)"))
  (bind (_returnvalue_roll _returnvalue_pitch _returnvalue_yaw) (`KismetMathLibrary.BreakRotator` (`KismetMathLibrary.FindLookAtRotation` (`SceneComponent.K2_GetComponentLocation` (`self.ActiveButton`)) (`SceneComponent.K2_GetComponentLocation` (`Actor.RootComponent` (`self.Girl`))))))
  (`SceneComponent.K2_SetRelativeRotation` (`self.ActiveButton`) (`KismetMathLibrary.MakeRotator` 0.0 0.0 _returnvalue_yaw) false false))

(event `self.ReceiveBeginPlay`
  (bind _outactors (`GameplayStatics.GetAllActorsOfClass` "/Game/Liemander_Core/Blueprints/BP_AngryFrog.BP_AngryFrog_C"))
  (set `self.Target Frog` (`|GetArrayItem` _outactors))
  (bind _outactors_2 (`GameplayStatics.GetAllActorsOfClass` "/Game/Liemander_Core/MainGirl/BP_MainGirl.BP_MainGirl_C"))
  (set `self.Girl` (`|GetArrayItem` _outactors_2))
  (bind _asbp_main_controller (cast `/Game/Liemander_Core/MainGirl/BP_MainController` (`GameplayStatics.GetPlayerController` 0)))
  (add `/Game/Liemander_Core/MainGirl/BP_MainController.ActivateButton` _asbp_main_controller (`|CreateDelegate` :!event `TryActivateButton`)))

(event `self.ButtonTrigger.OnComponentBeginOverlap`
  (params (OverlappedComponent :type "PrimitiveComponent Object Reference") (OtherActor :type "Actor Object Reference") (OtherComp :type "PrimitiveComponent Object Reference") (OtherBodyIndex :type Integer) (bFromSweep :type Boolean) (SweepResult :type "HitResult Structure (by ref)"))
  (cast `/Game/Liemander_Core/MainGirl/BP_MainGirl` OtherActor)
  (`SceneComponent.SetVisibility` (`self.ActiveButton`) true false)
  (set `self.CanActivateButton` true))

(event `self.ButtonTrigger.OnComponentEndOverlap`
  (params (OverlappedComponent :type "PrimitiveComponent Object Reference") (OtherActor :type "Actor Object Reference") (OtherComp :type "PrimitiveComponent Object Reference") (OtherBodyIndex :type Integer))
  (cast `/Game/Liemander_Core/MainGirl/BP_MainGirl` OtherActor)
  (`SceneComponent.SetVisibility` (`self.ActiveButton`) false false)
  (set `self.CanActivateButton` false))

(event `TryActivateButton`
  (bind _returnvalue (`self.K2_GetActorLocation`))
  (bind _target_frog (`self.Target Frog`))
  (bind _bp_healthcomponent (`/Game/Liemander_Core/Blueprints/BP_AngryFrog.BP_HealthComponent` (`self.Target Frog`)))
  (bind _returnvalue_location (`KismetMathLibrary.BreakTransform` (`SceneComponent.K2_GetComponentToWorld` (`/Game/Liemander_Core/Blueprints/BP_AngryFrog.SM_FrogBody` _target_frog))))
  (if (`self.CanActivateButton`)
    (set `self.isBroken` true)
    (`|ExecutionSequence`
      (:`then_0`
        (`/Game/Liemander_Core/Blueprints/BP_HealthComponent.Subtract health` _bp_healthcomponent 1)
        (if (== (`/Game/Liemander_Core/Blueprints/BP_HealthComponent.Health` _bp_healthcomponent) 0)
          (set `/Game/Liemander_Core/Blueprints/BP_AngryFrog.IsDead` true _target_frog)
          (`GameplayStatics.SpawnEmitterAtLocation` "/Game/StarterContent/Particles/P_Sparks.P_Sparks" _returnvalue_location (struct) (100.0 100.0 100.0))))
      (:`then_1`
        (`GameplayStatics.PlaySoundAtLocation` "/Game/Liemander_Core/Sounds/SW_TransformerBkoreExplotion_1.SW_TransformerBkoreExplotion_1" _returnvalue (struct) 2.0 1.0 0.0 null null null null)
        (`GameplayStatics.PlaySoundAtLocation` "/Game/Liemander_Core/Sounds/SW_TransformerBkoreElectro.SW_TransformerBkoreElectro" _returnvalue (struct) 0.6 1.0 0.0 null null null null)
        (`self.K2_DestroyActor`)))))

(fn `UserConstructionScript`)
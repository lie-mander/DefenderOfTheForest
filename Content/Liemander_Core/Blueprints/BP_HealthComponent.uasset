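; Actor health component that stores a Health value and reports damage and death through HCTakingDamage and HCDead calls.
; SubtractHealth lowers Health and signals damage, while SetHealth overwrites the value directly.
; Both signal death only when Health equals exactly zero, with no clamping, and PrintHealth prints the value with a supplied name for debugging.
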(fn `Print health`
  (params (Name :type String))
  (`KismetSystemLibrary.PrintString` (`KismetStringLibrary.Concat_StrStr` Name " has health: " (`KismetStringLibrary.Conv_IntToString` (`self.Health`)))))

(fn `Set health`
  (params (NewParam :type Integer))
  (set `self.Health` NewParam)
  (if (== (`self.Health`) 0)
    (`self.HC_Dead`)))

(fn `Subtract health`
  (params (`To subtract` :type Integer))
  (set `self.Health` (- (`self.Health`) `To subtract`))
  (`self.HC_TakingDamage`)
  (if (== (`self.Health`) 0)
    (`self.HC_Dead`)))
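; BP_FallingRail is a rail hazard that breaks and falls after the player character, BP_MainGirl, enters its trigger volume.
; The Trigger overlap plays a cracking sound, waits briefly, then enables physics on both Rail and Trigger with a quieter breaking sound.
; Any overlap on the Rail plays a destruction sound and destroys the actor.
; The construction script hides the Trigger.
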(event `self.Trigger.OnComponentBeginOverlap`
  (params (OverlappedComponent :type "PrimitiveComponent Object Reference") (OtherActor :type "Actor Object Reference") (OtherComp :type "PrimitiveComponent Object Reference") (OtherBodyIndex :type Integer) (bFromSweep :type Boolean) (SweepResult :type "HitResult Structure (by ref)"))
  (cast `/Game/Liemander_Core/MainGirl/BP_MainGirl` OtherActor)
  (`GameplayStatics.PlaySoundAtLocation` "/Game/Liemander_Core/Sounds/SW_StartRailBroking.SW_StartRailBroking" (`SceneComponent.K2_GetComponentLocation` (`self.Rail`)) (struct) 0.2 1.0 0.0 null null null null)
  (`KismetSystemLibrary.Delay` 1.7)
  (`PrimitiveComponent.SetSimulatePhysics` (`self.Rail`) true)
  (`PrimitiveComponent.SetSimulatePhysics` (`self.Trigger`) true)
  (`GameplayStatics.PlaySoundAtLocation` "/Game/Liemander_Core/Sounds/SW_RailBroking.SW_RailBroking" (`SceneComponent.K2_GetComponentLocation` (`self.Rail`)) (struct) 0.2 1.0 0.0 null null null null))

(event `self.Rail.OnComponentBeginOverlap`
  (params (OverlappedComponent :type "PrimitiveComponent Object Reference") (OtherActor :type "Actor Object Reference") (OtherComp :type "PrimitiveComponent Object Reference") (OtherBodyIndex :type Integer) (bFromSweep :type Boolean) (SweepResult :type "HitResult Structure (by ref)"))
  (`GameplayStatics.PlaySoundAtLocation` "/Game/Liemander_Core/Sounds/SW_RailDestroy.SW_RailDestroy" (`SceneComponent.K2_GetComponentLocation` (`self.Rail`)) (struct) 1.0 1.0 0.0 null null null null)
  (`self.K2_DestroyActor`))

(fn `UserConstructionScript`
  (`SceneComponent.SetVisibility` (`self.Trigger`) false false))
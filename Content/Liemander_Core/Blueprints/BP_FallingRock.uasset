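; BP_FallingRock is a falling-rock trap that drops when BP_MainGirl enters its trigger, which is hidden by the construction script.
; The trigger overlap enables physics on the rock and plays a falling sound.
; When the rock later overlaps, it plays an impact sound, sphere-traces around itself to subtract health from BP_MainGirl if hit, then destroys the actor.
; The impact's cast tests the actor's own Trigger component rather than what was overlapped.
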(event `self.Trigger.OnComponentBeginOverlap`
  (params (OverlappedComponent :type "PrimitiveComponent Object Reference") (OtherActor :type "Actor Object Reference") (OtherComp :type "PrimitiveComponent Object Reference") (OtherBodyIndex :type Integer) (bFromSweep :type Boolean) (SweepResult :type "HitResult Structure (by ref)"))
  (cast `/Game/Liemander_Core/MainGirl/BP_MainGirl` OtherActor)
  (`PrimitiveComponent.SetSimulatePhysics` (`self.Rock`) true)
  (`GameplayStatics.PlaySoundAtLocation` "/Game/Liemander_Core/Sounds/SW_StartRockFalling.SW_StartRockFalling" (`SceneComponent.K2_GetComponentLocation` (`self.Rock`)) (struct) 0.2 1.0 0.0 null null null null))

(event `self.Rock.OnComponentBeginOverlap`
  (params (OverlappedComponent :type "PrimitiveComponent Object Reference") (OtherActor :type "Actor Object Reference") (OtherComp :type "PrimitiveComponent Object Reference") (OtherBodyIndex :type Integer) (bFromSweep :type Boolean) (SweepResult :type "HitResult Structure (by ref)"))
  (bind _returnvalue (`SceneComponent.K2_GetComponentLocation` (`self.Rock`)))
  (cast `MeshComponent` (`self.Trigger`))
  (bind _outhit (`KismetSystemLibrary.SphereTraceSingleForObjects` _returnvalue _returnvalue 200.0 (`self.Object Types`)))
  (`GameplayStatics.PlaySoundAtLocation` "/Game/Liemander_Core/Sounds/SW_EndingRockFalling.SW_EndingRockFalling" (`SceneComponent.K2_GetComponentLocation` (`self.Rock`)) (struct) 0.3 1.0 0.0 null null null null)
  (bind _asbp_main_girl (cast `/Game/Liemander_Core/MainGirl/BP_MainGirl` (`.HitActor` (`GameplayStatics.BreakHitResult` _outhit)))
    (:`then`
      (`/Game/Liemander_Core/Blueprints/BP_HealthComponent.Subtract health` (`/Game/Liemander_Core/MainGirl/BP_MainGirl.BP_HealthComponent` _asbp_main_girl) 1)
      (`self.K2_DestroyActor`))
    (:`CastFailed`
      (`self.K2_DestroyActor`))))

(fn `UserConstructionScript`
  (`SceneComponent.SetVisibility` (`self.Trigger`) false false))
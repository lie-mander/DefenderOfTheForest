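; End-game trigger volume that plays the final frog explosion and ends the game when BP_MainGirl enters it while armed.
; BeginPlay binds to the health-component death event of the first BP_AngryFrog, and ActivateTrigger arms the volume.
; Overlap binds the ending screen on WBP_Respawning, blends the camera to this actor, then uses delays to sequence explosion effects at the frog and CallEndGame.
; The armed flag clears only after both delays.
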(event `self.ReceiveBeginPlay`
  (bind _outactors (`GameplayStatics.GetAllActorsOfClass` "/Game/Liemander_Core/Blueprints/BP_AngryFrog.BP_AngryFrog_C"))
  (bind _output (`|GetArrayItem` _outactors))
  (set `self.Frog` _output)
  (add `/Game/Liemander_Core/Blueprints/BP_HealthComponent.HC_Dead` (`/Game/Liemander_Core/Blueprints/BP_AngryFrog.BP_HealthComponent` _output) (`|CreateDelegate` :!event `ActivateTrigger`)))

(event `ActivateTrigger`
  (set `self.CanActivate` true))

(event `self.Trigger.OnComponentBeginOverlap`
  (params (OverlappedComponent :type "PrimitiveComponent Object Reference") (OtherActor :type "Actor Object Reference") (OtherComp :type "PrimitiveComponent Object Reference") (OtherBodyIndex :type Integer) (bFromSweep :type Boolean) (SweepResult :type "HitResult Structure (by ref)"))
  (bind _returnvalue (`SceneComponent.K2_GetComponentLocation` (`Actor.RootComponent` (`self.Frog`))))
  (cast `/Game/Liemander_Core/MainGirl/BP_MainGirl` OtherActor)
  (if (`self.CanActivate`)
    (bind _foundwidgets (`WidgetBlueprintLibrary.GetAllWidgetsOfClass` "/Game/Liemander_Core/Widgets/WBP_Respawning.WBP_Respawning_C"))
    (`/Game/Liemander_Core/Widgets/WBP_Respawning.BindEndingScreen` (`|GetArrayItem` _foundwidgets))
    (bind _returnvalue_2 (`GameplayStatics.GetActorOfClass` "BP_FinalTrigger_C"))
    (`PlayerController.SetViewTargetWithBlend` (`GameplayStatics.GetPlayerController` 0) _returnvalue_2 1.0 "VTBlend_Linear" 0.0 false)
    (`KismetSystemLibrary.Delay` 2.0)
    (`GameplayStatics.PlaySoundAtLocation` "/Game/Liemander_Core/Sounds/SW_FrogExplotion_2.SW_FrogExplotion_2" _returnvalue (struct) 1.0 1.0 0.0 null null null null)
    (`GameplayStatics.SpawnEmitterAtLocation` "/Game/StarterContent/Particles/P_Explosion.P_Explosion" _returnvalue (struct) (50.0 50.0 50.0))
    (`GameplayStatics.SpawnEmitterAtLocation` "/Game/StarterContent/Particles/P_Fire.P_Fire" _returnvalue (struct) (50.0 50.0 50.0))
    (`KismetSystemLibrary.Delay` 2.0)
    (`self.EndGame`)
    (set `self.CanActivate` false)))

(fn `UserConstructionScript`)
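; BP_SafeZone is an invisible volume that keeps BP_MainGirl safe from the angry frog's attacks.
; On BeginPlay it caches the first BP_AngryFrog in the level and turns its attack off.
; StaticMesh overlaps with BP_MainGirl disable the frog's attack on entry and re-enable it on exit.
; The construction script hides the mesh, leaving it to serve only as the trigger shape.
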(event `self.ReceiveBeginPlay`
  (bind _outactors (`GameplayStatics.GetAllActorsOfClass` "/Game/Liemander_Core/Blueprints/BP_AngryFrog.BP_AngryFrog_C"))
  (bind _output_get (set `self.Frog` (`|GetArrayItem` _outactors)))
  (set `/Game/Liemander_Core/Blueprints/BP_AngryFrog.isCanAttack` false _output_get))

(event `self.StaticMesh.OnComponentBeginOverlap`
  (params (OverlappedComponent :type "PrimitiveComponent Object Reference") (OtherActor :type "Actor Object Reference") (OtherComp :type "PrimitiveComponent Object Reference") (OtherBodyIndex :type Integer) (bFromSweep :type Boolean) (SweepResult :type "HitResult Structure (by ref)"))
  (cast `/Game/Liemander_Core/MainGirl/BP_MainGirl` OtherActor)
  (set `/Game/Liemander_Core/Blueprints/BP_AngryFrog.isCanAttack` false (`self.Frog`)))

(event `self.StaticMesh.OnComponentEndOverlap`
  (params (OverlappedComponent :type "PrimitiveComponent Object Reference") (OtherActor :type "Actor Object Reference") (OtherComp :type "PrimitiveComponent Object Reference") (OtherBodyIndex :type Integer))
  (cast `/Game/Liemander_Core/MainGirl/BP_MainGirl` OtherActor)
  (set `/Game/Liemander_Core/Blueprints/BP_AngryFrog.isCanAttack` true (`self.Frog`)))

(fn `UserConstructionScript`
  (`SceneComponent.SetVisibility` (`self.StaticMesh`) false false))
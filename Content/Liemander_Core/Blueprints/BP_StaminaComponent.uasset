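; Stamina component that tracks a CurrentStamina meter for the first BP_MainGirl found in the level.
; BeginPlay caches that actor and copies its MaxWalkSpeed into MaxStamina, which serves as both speed threshold and overload value.
; Each Tick adds a fixed step while velocity exactly equals MaxStamina, otherwise subtracts it or clamps at zero.
; It only prints "Stamina Overloaded" on exact equality with MaxStamina, with no upper clamp.
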(event `self.ReceiveBeginPlay`
  (bind _outactors (`GameplayStatics.GetAllActorsOfClass` "/Game/Liemander_Core/MainGirl/BP_MainGirl.BP_MainGirl_C"))
  (bind _output (`|GetArrayItem` _outactors))
  (set `self.MaxStamina` (`CharacterMovementComponent.MaxWalkSpeed` (`Character.CharacterMovement` _output)))
  (set `self.Girl` _output))

(event `self.ReceiveTick`
  (params (DeltaSeconds :type "Float (single-precision)"))
  (if (== (`KismetMathLibrary.VSize` (`Actor.GetVelocity` (`self.Girl`))) (`self.MaxStamina`))
    (set `self.CurrentStamina` (+ (`self.CurrentStamina`) 0.05))
    (if (== (`self.CurrentStamina`) (`self.MaxStamina`)) :!label _label
      (`KismetSystemLibrary.PrintString` "Stamina Overloaded"))
    (elif (<= (`self.CurrentStamina`) 0.0)
      (set `self.CurrentStamina` 0.0)
      (else
        (set `self.CurrentStamina` (+ (`self.CurrentStamina`) -0.05))
        (goto _label)))))
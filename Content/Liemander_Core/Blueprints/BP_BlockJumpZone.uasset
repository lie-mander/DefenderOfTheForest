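; BP_BlockJumpZone is an invisible trigger volume that stops the player from jumping while inside it.
; Its static mesh acts as the overlap shape and is hidden by the construction script.
; When BP_MainGirl begins or ends overlap, it sets CanJump on the first player's BP_MainController to false or true.
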(event `self.ReceiveBeginPlay`)

(event `self.StaticMesh.OnComponentBeginOverlap`
  (params (OverlappedComponent :type "PrimitiveComponent Object Reference") (OtherActor :type "Actor Object Reference") (OtherComp :type "PrimitiveComponent Object Reference") (OtherBodyIndex :type Integer) (bFromSweep :type Boolean) (SweepResult :type "HitResult Structure (by ref)"))
  (cast `/Game/Liemander_Core/MainGirl/BP_MainGirl` OtherActor)
  (bind _asbp_main_controller (cast `/Game/Liemander_Core/MainGirl/BP_MainController` (`GameplayStatics.GetPlayerController` 0)))
  (set `/Game/Liemander_Core/MainGirl/BP_MainController.CanJump` false _asbp_main_controller))

(event `self.StaticMesh.OnComponentEndOverlap`
  (params (OverlappedComponent :type "PrimitiveComponent Object Reference") (OtherActor :type "Actor Object Reference") (OtherComp :type "PrimitiveComponent Object Reference") (OtherBodyIndex :type Integer))
  (cast `/Game/Liemander_Core/MainGirl/BP_MainGirl` OtherActor)
  (bind _asbp_main_controller (cast `/Game/Liemander_Core/MainGirl/BP_MainController` (`GameplayStatics.GetPlayerController` 0)))
  (set `/Game/Liemander_Core/MainGirl/BP_MainController.CanJump` true _asbp_main_controller))

(fn `UserConstructionScript`
  (`SceneComponent.SetVisibility` (`self.StaticMesh`) false false))